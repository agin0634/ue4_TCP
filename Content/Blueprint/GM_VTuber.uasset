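; GM_VTuber, apparently a game mode, drives a TCP server hosted in the GI_TCPServer game instance.
; On BeginPlay it creates a socket on a hard-coded LAN address and port, then calls accept if creation succeeds.
; Each Tick it receives from the socket while the accept flag is set and only prints the data on screen for debugging.
; EndPlay closes the socket.
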(event `self.ReceiveBeginPlay`
  (bind _asgi_tcpserver (cast `/Game/Blueprint/GI_TCPServer` (`GameplayStatics.GetGameInstance`)))
  (set `self.GameInstanceRef` _asgi_tcpserver)
  (bind _returnvalue (`TCPSocketInstance.createSoc` _asgi_tcpserver "192.168.11.242" 1999 1))
  (if _returnvalue
    (`TCPSocketInstance.acceptSoc` _asgi_tcpserver)))

(event `self.ReceiveEndPlay`
  (params (EndPlayReason :type "EEndPlayReason Enum" :default "Destroyed"))
  (`TCPSocketInstance.closeSoc` (`self.GameInstanceRef`)))

(event `self.ReceiveTick`
  (params (DeltaSeconds :type "Float (single-precision)"))
  (bind _gameinstanceref (`self.GameInstanceRef`))
  (if (`TCPSocketInstance.bIsAccept` _gameinstanceref)
    (bind _returnvalue (`TCPSocketInstance.recvSoc` _gameinstanceref))
    (`KismetSystemLibrary.PrintString` _returnvalue true true (struct :`G` 0.66 :`B` 1.0 :`A` 1.0) 10.0)))

(fn `UserConstructionScript`)